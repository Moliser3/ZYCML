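; Test-mode player controller for click-to-move control of an AI hero, which it spawns at a fixed location on BeginPlay.
; It shows the cursor and has GM_TEST attach the camera to the hero's spring arm.
; Left-click release traces under the cursor, draws a debug box, makes the hero gaze at NPCs or rotate when running, then temporarily calls move-to-point.
; Left Shift toggles running and walking.
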(event `self.ReceiveBeginPlay`
  (`|ExecutionSequence`
    (:`then_0`
      (set `self.bShowMouseCursor` true) ; 鼠标显示
    )
    (:`then_1`
      (`self.SpawnHero`) ; 生成控制角色
    )
    (:`then_2`
      (`self.SetCameraToCtrAi`) ; 设置相机位置
    )))

(event `MouseLeftOnClick`
  (`self.MouseHit`))

(event `SetCameraToCtrAi`
  (bind _asgm_test (cast `/Game/CoreSystem/TESTMode/GM_TEST` (`GameplayStatics.GetGameMode`)))
  (`/Game/CoreSystem/TESTMode/GM_TEST.AttachCameraToComp` _asgm_test (`/Game/CoreSystem/BP_AIHero.SpringArm` (`self.Hero`))))

(event `Key|LeftMouseButton`
  (params (Key :type "Key Structure"))
  ; 控制输入
  (:`Released`
    (`self.MouseLeftonClick`)))

(event `MouseHit`
  (bind (_bblockinghit _binitialoverlap _time _distance _location _impactpoint _normal _impactnormal _physmat _hitactor) (`GameplayStatics.BreakHitResult` (`self.GetHitResultUnderCursorByChannel` "TraceTypeQuery1")))
  ; 鼠标点击事件
  (`KismetSystemLibrary.DrawDebugBox` _location (5.0 5.0 5.0) (struct :`R` 0.286987 :`G` 1.0 :`A` 1.0) (struct) 10.0)
  (`self.CheckTargetType` _hitactor)
  (`/Game/CoreSystem/BP_AIHero.MoveToTargetPos` (`self.Hero`) _location :!pinned true) ; 临时调用：角色移动
)

(event `Key|LeftShift`
  (params (Key :type "Key Structure"))
  ; 控制输入
  (:`Pressed`
    (set `self.NexMoveState` "Running")
    (`/Game/CoreSystem/BP_AIHero.SetUseMoveState` (`self.Hero`) (`self.NexMoveState`) :!label _label))
  (:`Released`
    (set `self.NexMoveState` "Walking")
    (goto _label)))

(event `Key|One`
  (params (Key :type "Key Structure"))
  ; 控制输入
)

(event `Key|Two`
  (params (Key :type "Key Structure"))
  ; 控制输入
)

(fn `CheckTargetType`
  (params (HitActor :type "Actor Object Reference"))
  (`/Engine/EditorBlueprintResources/StandardMacros.IsValid` HitActor
    (:`Is Valid`
      (bind _asbase_character (cast `BaseCharacter` (`local.HitActor`))
        (:`then`
          (switch `ECharacterType` (`BaseCharacter.CharacterType` _asbase_character)
            (:`Player`
              (if (`|EnumEquality` (`self.NexMoveState`) "Running") :!label _label
                (`IHolderFunction.ActivateRotating` (`self.Hero`))))
            (:`NPC`
              (`BaseCharacter.SetTargetActor` (`self.Hero`) _asbase_character)
              (`IHolderFunction.ActiveGazing` (`self.Hero`)))))
        (:`CastFailed`
          (goto _label))))))

(fn `SpawnHero`
  (bind _returnvalue (`|SpawnActorFromClass` "/Game/CoreSystem/BP_AIHero.BP_AIHero_C" (`KismetMathLibrary.MakeTransform` (-100.0 -545.0 100.0)) "Undefined" "MultiplyWithRoot" null null))
  (`/Engine/EditorBlueprintResources/StandardMacros.IsValid` _returnvalue
    (:`Is Valid`
      (set `self.Hero` _returnvalue))))

(fn `UserConstructionScript`)