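; GM_TEST is a test game mode that sets up the main camera for the player.
; On BeginPlay it spawns BP_MainCamera at a fixed, downward-angled transform, stores it and makes it the first player controller's view target.
; AttachCameraToComp can attach that camera to a supplied spring arm component, snapping its rotation and zeroing its relative location.
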(event `self.ReceiveBeginPlay`
  (`self.SpawnCamera`))

(event `SpawnCamera`
  (bind _returnvalue (`|SpawnActorFromClass` "/Game/CoreSystem/BP_MainCamera.BP_MainCamera_C" (`KismetMathLibrary.MakeTransform` (-1250.0 -954.0 1369.0) (struct :`Pitch` -50.0 :`Yaw` 50.0)) "Undefined" "MultiplyWithRoot" null null))
  (`/Engine/EditorBlueprintResources/StandardMacros.IsValid` _returnvalue
    (:`Is Valid`
      (set `self.MainCamera` _returnvalue)
      (`PlayerController.SetViewTargetWithBlend` (`GameplayStatics.GetPlayerController` 0) _returnvalue 0.0 "VTBlend_Linear" 0.0 false))))

(fn `AttachCameraToComp`
  (params (SpringArmCom :type "SpringArmComponent Object Reference"))
  (`self.K2_AttachToComponent` (`self.MainCamera`) SpringArmCom "None" "KeepRelative" "SnapToTarget" "KeepRelative" true)
  (`self.K2_SetActorRelativeLocation` (`self.MainCamera`) (0.0 0.0 0.0) false false))

(fn `UserConstructionScript`)