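; BP_AIHero is an AI-controlled hero character that moves to target positions and keeps its animation in step with its behavior.
; On BeginPlay it possesses itself with its AI controller, caches its ABP_Character anim instance and binds to OnBehaviorChanged, unbinding on Destroyed.
; RefreshBPAMovement pushes behavior and move state into the anim instance.
; MoveToTargetPos wraps AI MoveTo between BeginActiveMove and OnMoveEnd, the latter firing only on success.
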(event `self.ReceiveBeginPlay`
  (`|ExecutionSequence`
    (:`then_0`
      (`self.GetCtr`))
    (:`then_1`
      (`self.GetAnimInstance`))))

(event `self.ReceiveActorBeginOverlap`
  (params (OtherActor :type "Actor Object Reference")))

(event `self.ReceiveTick`
  (params (DeltaSeconds :type "Float (single-precision)")))

(event `GetAnimInstance`
  (bind _asabp_character (cast `/Game/CoreSystem/Animation/Character/ABP_Character` (`SkeletalMeshComponent.GetAnimInstance` (`self.Mesh`))))
  (set `self.BPAnimation` _asabp_character)
  (add `self.OnBehaviorChanged` (`|CreateDelegate` :!event `RefreshBPAMovement`)))

(event `GetCtr`
  (bind _returnvalue (`AIBlueprintHelperLibrary.GetAIController` self))
  (`/Engine/EditorBlueprintResources/StandardMacros.IsValid` _returnvalue
    (:`Is Valid`
      (bind _output_get (set `self.AICTR` _returnvalue))
      (`Controller.Possess` _output_get self))
    (:`Is Not Valid`
      (`KismetSystemLibrary.PrintString` "AICtr Is Null"))))

(event `MoveToTargetPos`
  (params (AIMoveTo :type "Vector Structure"))
  (`self.BeginActiveMove` self)
  (`|AIMoveTo` self AIMoveTo null
    (:`OnSuccess`
      (`self.OnMoveEnd`))))

(event `RefreshBPAMovement` :!signature `self.OnBehaviorChanged`
  (params (CurrentBehavior :type "ECharacterBehavior Enum" :default "Idle") (CurrentMoveState :type "EMoveState Enum" :default "Walking"))
  (bind _bpanimation (`self.BPAnimation`))
  (`/Engine/EditorBlueprintResources/StandardMacros.IsValid` _bpanimation
    (:`Is Valid`
      (`/Game/CoreSystem/Animation/Character/ABP_Character.SetMovement` _bpanimation CurrentBehavior)
      (`/Game/CoreSystem/Animation/Character/ABP_Character.SetMove` (`self.BPAnimation`) CurrentMoveState))))

(event `self.ReceiveDestroyed`
  (clear `self.OnBehaviorChanged`))

(fn `UserConstructionScript`)