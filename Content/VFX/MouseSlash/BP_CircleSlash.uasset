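; Circle slash VFX actor that plays a timed, material-driven slash effect at a given position.
; BeginPlay puts a dynamic instance of M_CircleSlash on the CircleSlash component.
; EnableSlash, meant for external callers, moves the actor and starts a timer, ignoring calls while a slash is playing.
; Tick runs PlaySlash, which feeds elapsed time over duration into OneSlashProgressValue until the target time is reached.
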(event `self.ReceiveBeginPlay`
  (bind _returnvalue (`KismetMaterialLibrary.CreateDynamicMaterialInstance` "/Game/VFX/MouseSlash/M_CircleSlash.M_CircleSlash"))
  (bind _output_get (set `self.DMI_CircleSlash` _returnvalue))
  (`PrimitiveComponent.SetMaterial` (`self.CircleSlash`) 0 _output_get))

(event `self.ReceiveTick`
  (params (DeltaSeconds :type "Float (single-precision)"))
  (`self.PlaySlash` DeltaSeconds))

(event `EnableSlash`
  (params (SlashTime :type "Float (double-precision)") (Pos :type "Vector Structure"))
  (if (not (`self.IsPlaySlash`))
    (`self.K2_SetActorLocation` Pos)
    (set `self.TargetTime` SlashTime)
    (set `self.IsPlaySlash` true)
    (set `self.CurrentTime` 0.0)))

(event `PlaySlash`
  (params (DelatTime :type "Float (double-precision)"))
  (if (`self.IsPlaySlash`)
    (`MaterialInstanceDynamic.SetScalarParameterValue` (`self.DMI_CircleSlash`) "OneSlashProgressValue" (/ (`self.CurrentTime`) (`self.TargetTime`)))
    (if (>= (`self.CurrentTime`) (`self.TargetTime`))
      (set `self.IsPlaySlash` false)
      (else
        (set `self.CurrentTime` (+ (`self.CurrentTime`) DelatTime))))))

(fn `UserConstructionScript`)